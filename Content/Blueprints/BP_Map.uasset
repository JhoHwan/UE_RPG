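; BP_Map is a map actor that generates a flat, square grid of blocks.
; Its construction script runs nested loops over WidthHieght, adding one InstancedStaticMesh instance per cell, spaced by BlockSize.
; Each instance has a fixed uniform scale and sits half a BlockSize below the actor's origin.
; The event graph holds only empty default events, so the Blueprint adds no runtime logic.
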(fn `UserConstructionScript`
  (bind _blocksize (`self.BlockSize`))
  (for _index (range (+ (`self.WidthHieght`) 1))
    (for _index_2 (range (+ (`self.WidthHieght`) 1))
      (`InstancedStaticMeshComponent.AddInstance` (`self.InstancedStaticMesh`) (`KismetMathLibrary.MakeTransform` (`KismetMathLibrary.MakeVector` (`KismetMathLibrary.Conv_IntToDouble` (* _index _blocksize)) (`KismetMathLibrary.Conv_IntToDouble` (* _index_2 _blocksize)) (`KismetMathLibrary.Conv_IntToDouble` (/ (`self.BlockSize`) -2))) (struct) (1.5 1.5 1.5)) false))))