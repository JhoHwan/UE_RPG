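; Player controller for the title screen that shows the mouse cursor and displays the title UI widget on begin play.
; On its LoginSuccess event it creates the fade widget if needed, adds it to the viewport and plays a fade-out animation.
; After a one-second delay it opens the CharacterSelect level.
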(event `self.ReceiveBeginPlay`
  (set `self.bShowMouseCursor` true)
  (bind _returnvalue (`|CreateWidget` "/Game/Blueprints/WBP/Title/WBP_Title.WBP_Title_C"))
  (bind _output_get (set `self.TitleWidget` _returnvalue))
  (`UserWidget.AddToViewport` _output_get 0))

(event `Login Success`
  (`|ExecutionSequence`
    (:`then_0`
      (`self.FadeWidget`
        (:`then`
          _)
        (:`else`
          (bind _returnvalue (`|CreateWidget` "/Game/Blueprints/WBP/WBP_FadeWidget.WBP_FadeWidget_C"))
          (set `self.FadeWidget` _returnvalue)))
      (`UserWidget.AddToViewport` (`self.FadeWidget`) 1)
      (`/Game/Blueprints/WBP/WBP_FadeWidget.PlayFadeOutAnim` (`self.FadeWidget`)))
    (:`then_1`
      (`KismetSystemLibrary.Delay` 1.0)
      (`GameplayStatics.OpenLevel` "CharacterSelect"))))

(fn `UserConstructionScript`)