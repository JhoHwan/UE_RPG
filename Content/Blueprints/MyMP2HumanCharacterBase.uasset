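; MyMP2HumanCharacterBase is a human character base Blueprint that dresses the character in gear when play begins.
; For the Male gender, its AppearanceComponent receives default cloth, gloves, pants and shoes data assets, then applies the appearance.
; After a short delay it equips a test cap without calling the general appearance update again.
; No other gender is handled, and the construction script is empty.
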(event `self.ReceiveBeginPlay`
  (bind _appearancecomponent (`self.AppearanceComponent`))
  (bind _appearancecomponent_2 (`self.AppearanceComponent`))
  (switch `EGenderType` (`self.Gender`)
    (:`Male`
      (`MP2CharacterAppearanceComponent.ChangeGearAppearance` _appearancecomponent "Cloth" "/Game/Items/Gear/DA_CL_Default.DA_CL_Default")
      (`MP2CharacterAppearanceComponent.ChangeGearAppearance` _appearancecomponent "Gloves" "/Game/Items/Gear/DA_GL_Default.DA_GL_Default")
      (`MP2CharacterAppearanceComponent.ChangeGearAppearance` _appearancecomponent_2 "Pants" "/Game/Items/Gear/DA_PA_Default.DA_PA_Default")
      (`MP2CharacterAppearanceComponent.ChangeGearAppearance` _appearancecomponent_2 "Shoes" "/Game/Items/Gear/DA_SH_Default.DA_SH_Default")
      (`MP2CharacterAppearanceComponent.ChangeAppearance` (`self.AppearanceComponent`) null)
      (`KismetSystemLibrary.Delay` 2.0)
      (`MP2CharacterAppearanceComponent.ChangeGearAppearance` (`self.AppearanceComponent`) "Cap" "/Game/Items/Gear/DA_CP_TestCap.DA_CP_TestCap"))))

(fn `UserConstructionScript`)