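; BP_BackPlane is an actor that keeps itself positioned in front of the player camera, at a set distance along its view direction.
; It caches player 0's camera manager on BeginPlay, then every Tick moves to the camera location plus its forward vector scaled by TargetDist, without sweep.
; A node to match the camera's rotation exists but is disconnected, so only location follows the camera.
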(event `self.ReceiveBeginPlay`
  (set `self.CamManager` (`GameplayStatics.GetPlayerCameraManager` 0)))

(event `self.ReceiveTick`
  (params (DeltaSeconds :type "Float (single-precision)"))
  (bind _cammanager (`self.CamManager`))
  (`self.K2_SetActorLocation` (+ (`PlayerCameraManager.GetCameraLocation` _cammanager) (* (`KismetMathLibrary.GetForwardVector` (`PlayerCameraManager.GetCameraRotation` _cammanager)) (`self.TargetDist`)))))

(fn `UserConstructionScript`)