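; BP_TestPlayer is a test player Blueprint that exercises character appearance changes through its AppearanceComponent.
; On BeginPlay, the Male gender case equips clothing, gloves, pants and shoes from data assets and applies a hair asset.
; Timed delays then recolor the hair pink and add a test cap, demonstrating runtime appearance swapping.
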(event `self.ReceiveBeginPlay`
  (bind _appearancecomponent (`self.AppearanceComponent`))
  (bind _appearancecomponent_2 (`self.AppearanceComponent`))
  (bind _appearancecomponent_3 (`self.AppearanceComponent`))
  (switch `EGenderType` (`self.Gender`)
    (:`Male`
      (`MP2CharacterAppearanceComponent.ChangeGearAppearance` _appearancecomponent "Cloth" "/Game/Items/Gear/DA_CL_Test.DA_CL_Test")
      (`MP2CharacterAppearanceComponent.ChangeGearAppearance` _appearancecomponent "Gloves" "/Game/Items/Gear/DA_GL_Default.DA_GL_Default")
      (`MP2CharacterAppearanceComponent.ChangeGearAppearance` _appearancecomponent_2 "Pants" "/Game/Items/Gear/DA_PA_Default.DA_PA_Default")
      (`MP2CharacterAppearanceComponent.ChangeGearAppearance` _appearancecomponent_2 "Shoes" "/Game/Items/Gear/DA_SH_Default.DA_SH_Default")
      (`MP2CharacterAppearanceComponent.ChangeAppearance` (`self.AppearanceComponent`) "/Game/Items/OutFit/DA_HR_Defualt.DA_HR_Defualt")
      (`KismetSystemLibrary.Delay` 3.0)
      (`MP2CharacterAppearanceComponent.ChangeHairColor` _appearancecomponent_3 (struct :`R` 1.0 :`G` 0.213849 :`B` 0.846024 :`A` 1.0))
      (`KismetSystemLibrary.Delay` 3.0)
      (`MP2CharacterAppearanceComponent.ChangeGearAppearance` _appearancecomponent_3 "Cap" "/Game/Items/Gear/DA_CP_TestCap.DA_CP_TestCap"))))

(fn `UserConstructionScript`)